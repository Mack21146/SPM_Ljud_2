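; BP_Door is an ambient door that periodically swings open and shut by itself with sound.
; A self-restarting loop begun at BeginPlay waits a random interval, then triggers the animation.
; One timeline lerps the mesh's yaw open while the audio component plays the door sound.
; After a random pause, a second timeline swings it back with the closing sound.
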(event Custom|Begin%20animation
  (bind _audio (Variables|Default|GetAudio))
  (bind _audio_2 (Variables|Default|GetAudio))
  (Audio|Components|Audio|SetSound _audio_2 "/Game/Audio/SoundFX/Door/SW_Door.SW_Door")
  (Audio|Components|Audio|Play _audio_2 0.0)
  (bind _move (Timeline|Timeline PlayFromStart)
    (:Update
      (Transformation|SetRelativeRotation (Variables|Default|GetStaticMesh) (Math|Rotator|MakeRotator 0.0 0.0 (Math|Float|Lerp 0.0 -4e+01 _move)) false false))
    (:Finished
      (Utilities|FlowControl|Delay (Math|Random|RandomFloatinRange 1.0 5.0))
      (Audio|Components|Audio|SetSound _audio "/Game/Audio/SoundFX/Door/SW_DoorClosing.SW_DoorClosing")
      (Audio|Components|Audio|Play _audio 0.0)
      (bind _move_2 (Timeline|Timeline_0 PlayFromStart)
        (:Update
          (Transformation|SetRelativeRotation (Variables|Default|GetStaticMesh) (Math|Rotator|MakeRotator 0.0 0.0 (Math|Float|Lerp -4e+01 0.0 _move_2)) false false))))))

(event Custom|Start%20loop
  (Utilities|FlowControl|Delay (Math|Random|RandomFloatinRange 15.0 3e+01))
  (CallFunction|BeginAnimation)
  (CallFunction|StartLoop))

(event EventBeginPlay
  (CallFunction|StartLoop))

(fn ConstructionScript)