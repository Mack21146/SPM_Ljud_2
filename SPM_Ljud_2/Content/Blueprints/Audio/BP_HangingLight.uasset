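; Hanging light Blueprint that periodically swings a component named Audio and plays a sound.
; From BeginPlay, a self-calling loop event waits a random delay, then triggers the animation without waiting for it to finish.
; Two chained timelines pitch the component out and back through a small angle, each preceded by the hanging light sound played at world origin rather than the actor's location.
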(event Custom|Begin%20animation
  (Audio|PlaySoundatLocation "/Game/Audio/SoundCues/SC_HangingLight.SC_HangingLight" "0, 0, 0" "0, 0, 0" 1.0 1.0 0.0 0 0 0 0)
  (bind _move (Timeline|Timeline PlayFromStart)
    (:Update
      (Transformation|SetRelativeRotation (Variables|Default|GetAudio) (Math|Rotator|MakeRotator 0.0 (Math|Float|Lerp 0.0 8.0 _move) 0.0) false false))
    (:Finished
      (Audio|PlaySoundatLocation "/Game/Audio/SoundCues/SC_HangingLight.SC_HangingLight" "0, 0, 0" "0, 0, 0" 1.0 1.0 0.0 0 0 0 0)
      (bind _move_2 (Timeline|Timeline_0 PlayFromStart)
        (:Update
          (Transformation|SetRelativeRotation (Variables|Default|GetAudio) (Math|Rotator|MakeRotator 0.0 (Math|Float|Lerp 8.0 0.0 _move_2) 0.0) false false))))))

(event Custom|Start%20loop
  (Utilities|FlowControl|Delay (Math|Random|RandomFloatinRange 1e+01 3e+01))
  (CallFunction|BeginAnimation)
  (CallFunction|StartLoop))

(event EventBeginPlay
  (CallFunction|StartLoop))

(fn ConstructionScript)