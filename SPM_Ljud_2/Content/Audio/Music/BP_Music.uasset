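; BP_Music is an actor that crossfades between outside and inside music as the third-person character crosses its overlap bounds.
; BeginPlay enables input and starts the outside track through the same chain that overlap begin uses, fading out any inside track.
; Overlap end fades in the inside track and fades out the outside one.
; Each switch spawns a new 2D sound rather than reusing components.
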(event Collision|EventActorBeginOverlap
  (params (OtherActor :type Actor%20Object%20Reference))
  (Utilities|Casting|CastToBP_ThirdPersonCharacter OtherActor)
  (bind _returnvalue (Audio|SpawnSound2D "/Game/Audio/Music/SW_MusicOutside.SW_MusicOutside" 1.0 1.0 0.0 0))
  (Audio|Components|Audio|FadeIn _returnvalue 0.0 1.0 0.0 "Linear" :!class /Script/Engine.AudioComponent)
  (Audio|Components|Audio|FadeOut (stale Collision|EventActorEndOverlap _returnvalue) 1.0 0.0 "Linear" :!class /Script/Engine.AudioComponent))

(event Collision|EventActorEndOverlap
  (params (OtherActor :type Actor%20Object%20Reference))
  (Utilities|Casting|CastToBP_ThirdPersonCharacter OtherActor)
  (bind _returnvalue (Audio|SpawnSound2D "/Game/Audio/Music/SW_MusicInside.SW_MusicInside" 1.0 1.0 0.0 0))
  (Audio|Components|Audio|FadeIn _returnvalue 1.0 1.0 0.0 "Linear" :!class /Script/Engine.AudioComponent)
  (Audio|Components|Audio|FadeOut (stale Collision|EventActorBeginOverlap _returnvalue) 1.0 0.0 "Linear" :!class /Script/Engine.AudioComponent))

(event EventBeginPlay
  (Input|EnableInput (Game|GetPlayerController 0))
  (bind _returnvalue (Audio|SpawnSound2D "/Game/Audio/Music/SW_MusicOutside.SW_MusicOutside" 1.0 1.0 0.0 0))
  (Audio|Components|Audio|FadeIn _returnvalue 0.0 1.0 0.0 "Linear" :!class /Script/Engine.AudioComponent)
  (Audio|Components|Audio|FadeOut (stale Collision|EventActorEndOverlap _returnvalue) 1.0 0.0 "Linear" :!class /Script/Engine.AudioComponent))

(fn ConstructionScript)